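; A cardboard target stand that rolls its target through a timeline started on BeginPlay and tracks damage against its Health.
; At zero health it increments the first-person character's Score, raises RefChar's HighScore if beaten, then destroys itself.
; On a new high score it loads an existing save slot without writing back, or creates and saves a SaveScore object without copying the score into it.
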(event `self.ReceiveBeginPlay`
  (bind (_direction _rotation) (`Timeline|RotateTarget`)
    (:`Update`
      (`SceneComponent.K2_SetRelativeRotation` (`self.cardboard_target`) (`KismetMathLibrary.MakeRotator` _rotation) false false))))

(event `self.ReceiveAnyDamage`
  (params (Damage :type "Float (single-precision)") (DamageType :type "DamageType Object Reference") (InstigatedBy :type "Controller Object Reference") (DamageCauser :type "Actor Object Reference"))
  (bind _ref_char (`self.Ref Char`))
  (bind _output_get (set `self.Health` (- (`self.Health`) Damage)))
  (if (<= _output_get 0.0)
    (`|ExecutionSequence`
      (:`then_0`
        (bind _asbp_first_person_character (cast `/Game/FirstPerson/Blueprints/BP_FirstPersonCharacter` (`GameplayStatics.GetPlayerCharacter` 0)))
        (bind _score (`/Game/FirstPerson/Blueprints/BP_FirstPersonCharacter.Score` _asbp_first_person_character))
        (`/Engine/EditorBlueprintResources/StandardMacros.IncrementInt` _score
          (:`  `
            (if (> _score (`/Game/FirstPerson/Blueprints/BP_FirstPersonCharacter.HighScore` _ref_char))
              (set `/Game/FirstPerson/Blueprints/BP_FirstPersonCharacter.HighScore` _score _ref_char)
              (bind _returnvalue (`GameplayStatics.DoesSaveGameExist` (`self.SlotName`)))
              (if _returnvalue
                (bind _returnvalue_2 (`GameplayStatics.LoadGameFromSlot` (`self.SlotName`)))
                (bind _output_get_2 (set `self.SaverSubClass` _returnvalue_2))
                (cast `/Game/FirstPerson/Blueprints/SaveScore` _output_get_2)
                (else
                  (bind _returnvalue_3 (`GameplayStatics.CreateSaveGameObject` "/Game/FirstPerson/Blueprints/SaveScore.SaveScore_C"))
                  (bind _output_get_3 (set `self.SaverSubClass` _returnvalue_3))
                  (`GameplayStatics.SaveGameToSlot` _output_get_3 (`self.SlotName`))))))))
      (:`then_1`
        (`self.K2_DestroyActor`)))))

(fn `UserConstructionScript`)